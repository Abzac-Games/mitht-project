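; Component for a shaft group on the OMEGA40PL equipment prop, driving an interactable, animated shaft.
; On BeginPlay it caches the mesh's ABP_Shaft_1 anim instance and the BP_Shaft_1_SM state machine instance.
; Completing an interaction calls Act on that state machine.
; The construction script registers the mesh with the parent's mesh list, and the UI state shows the interaction action title.
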(event OnInteractionCompleted(Interactable)
  (params (FinishedInteractionType :type EInteractableType%20Enum :default "EIT_Hold") (FinishTime :type Float%20%28single-precision%29))
  (Default|Act (Variables|Default|GetState)))

(event EventBeginPlay
  (bind _asabp_shaft_1 (Utilities|Casting|CastToABP_Shaft_1 (Components|SkeletalMesh|GetAnimInstance (Variables|Default|GetMesh))))
  (Variables|Default|SetAnimation _asabp_shaft_1)
  (bind _asbp_shaft_1_sm (Utilities|Casting|CastToBP_Shaft_1_SM (Class|SMStateMachineComponent|GetInstance (Variables|Default|GetState%20Machine))))
  (Variables|Default|SetState _asbp_shaft_1_sm))

(fn ConstructionScript
  (Utilities|Array|Add (Variables|Default|GetMeshes) (Variables|Default|GetMesh))
  (|CallParentFunction))

(fn GetUIState
  (return (Utilities|Struct|MakeEquipmentComponentUIState (Class|ActorInteractableComponent|GetInteractionActionTitle (Variables|Default|GetInteractable)) "")))