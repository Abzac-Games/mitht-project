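; BP_Shaft_Group is a grouping Blueprint for the shaft assembly of the OMEGA40PL equipment prop, driving a pipe, a bolt and a shaft as one unit.
; On BeginPlay it casts the three child actors to their part Blueprints, stores the references and binds ActEvent to its OnAct dispatcher.
; Act fires that dispatcher, and ActEvent relays the call to each part's own Act.
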(event Custom|Act%20Event
  (Default|Act (Variables|Default|GetPipe%202))
  (Default|Act (Variables|Default|GetBolt%201))
  (Default|Act (Variables|Default|GetShaft%201)))

(event EventBeginPlay
  (bind _asbp_pipe_2 (Utilities|Casting|CastToBP_Pipe_2 (Variables|/Script/Engine.ChildActorComponent|GetChildActor (Variables|Default|GetPipe_2))))
  (Variables|Default|SetPipe%202 _asbp_pipe_2)
  (bind _asbp_bolt_1 (Utilities|Casting|CastToBP_Bolt_1 (Variables|/Script/Engine.ChildActorComponent|GetChildActor (Variables|Default|GetBolt_1))))
  (Variables|Default|SetBolt%201 _asbp_bolt_1)
  (bind _asbp_shaft_1 (Utilities|Casting|CastToBP_Shaft_1 (Variables|/Script/Engine.ChildActorComponent|GetChildActor (Variables|Default|GetShaft_1))))
  (Variables|Default|SetShaft%201 _asbp_shaft_1)
  (EventDispatchers|BindEventtoOnAct (delegate Custom|Act%20Event)))

(fn ConstructionScript)

(fn Act
  (Default|CallOnAct))