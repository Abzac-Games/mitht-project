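; BP_Button_1 is an interactable button component for the OMEGA40PL equipment prop.
; On BeginPlay it caches its mesh's animation instance and a BP_Button_1_SM state machine instance, and completing an interaction calls Press on that state machine.
; The construction script registers its mesh and shape with the parent's arrays.
; GetUIState returns the interaction action title with a placeholder "Hello World" state text.
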(event OnInteractionCompleted(Interactable)
  (params (FinishedInteractionType :type EInteractableType%20Enum :default "EIT_Hold") (FinishTime :type Float%20%28single-precision%29))
  (Default|Press (Variables|Default|GetState)))

(event EventBeginPlay
  (bind _asabp_button_1 (Utilities|Casting|CastToABP_Button_1 (Components|SkeletalMesh|GetAnimInstance (Variables|Default|GetMesh))))
  (Variables|Default|SetAnimation _asabp_button_1)
  (bind _asbp_button_1_sm (Utilities|Casting|CastToBP_Button_1_SM (Class|SMStateMachineComponent|GetInstance (Variables|Default|GetState%20Machine))))
  (Variables|Default|SetState _asbp_button_1_sm))

(fn ConstructionScript
  (Utilities|Array|Add (Variables|Default|GetMeshes) (Variables|Default|GetMesh))
  (Utilities|Array|Add (Variables|Default|GetShapes) (Variables|Default|GetShape))
  (|CallParentFunction))

(fn GetUIState
  (return (Utilities|Struct|MakeEquipmentComponentUIState (Class|ActorInteractableComponent|GetInteractionActionTitle (Variables|Default|GetInteractable)) (Utilities|Text|MakeLiteralText "Hello World"))))