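; Interactable sensor button component for the OMEGA40PL equipment prop.
; On begin play it caches its mesh animation instance and its state machine instance.
; A completed interaction triggers the state machine's press, and the UI name comes from the interactable's action title.
; The construction script registers its mesh and shape with the parent class.
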(event OnInteractionCompleted(Interactable)
  (params (FinishedInteractionType :type EInteractableType%20Enum :default "EIT_Hold") (FinishTime :type Float%20%28single-precision%29))
  (Default|Press (Variables|Default|GetState)))

(event EventBeginPlay
  (bind _asabp_sensor_button_003 (Utilities|Casting|CastToABP_Sensor_Button_003 (Components|SkeletalMesh|GetAnimInstance (Variables|Default|GetMesh))))
  (Variables|Default|SetAnimation _asabp_sensor_button_003)
  (bind _asbp_sensor_button_002_sm (Utilities|Casting|CastToBP_Sensor_Button_002_SM (Class|SMStateMachineComponent|GetInstance (Variables|Default|GetState%20Machine))))
  (Variables|Default|SetState _asbp_sensor_button_002_sm))

(fn ConstructionScript
  (Utilities|Array|Add (Variables|Default|GetMeshes) (Variables|Default|GetMesh))
  (Utilities|Array|Add (Variables|Default|GetShapes) (Variables|Default|GetShape))
  (|CallParentFunction))

(fn GetUIState
  (return (Utilities|Struct|MakeEquipmentComponentUIState (Class|ActorInteractableComponent|GetInteractionActionTitle (Variables|Default|GetInteractable)) "")))