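; BP_Switch_1_003 is an interactable switch prop for the OMEGA40PL equipment.
; On BeginPlay it caches its animation Blueprint instance from the mesh and its switch-specific state machine instance.
; A completed interaction is forwarded to that state machine through Interact.
; The construction script registers the mesh and shape in the Meshes and Shapes arrays before running the parent's construction.
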(event OnInteractionCompleted(Interactable)
  (params (FinishedInteractionType :type EInteractableType%20Enum :default "EIT_Hold") (FinishTime :type Float%20%28single-precision%29))
  (Default|Interact (Variables|Default|GetState)))

(event EventBeginPlay
  (bind _asabp_switch_1_003 (Utilities|Casting|CastToABP_Switch_1_003 (Components|SkeletalMesh|GetAnimInstance (Variables|Default|GetMesh))))
  (Variables|Default|SetAnimation _asabp_switch_1_003)
  (bind _asbp_switch_1_003_sm (Utilities|Casting|CastToBP_Switch_1_003_SM (Class|SMStateMachineComponent|GetInstance (Variables|Default|GetState%20Machine))))
  (Variables|Default|SetState _asbp_switch_1_003_sm))

(fn ConstructionScript
  (Utilities|Array|Add (Variables|Default|GetMeshes) (Variables|Default|GetMesh))
  (Utilities|Array|Add (Variables|Default|GetShapes) (Variables|Default|GetShape))
  (|CallParentFunction))