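; BP_Room_Door is an interactable room door that swings open and closed when the player completes an interaction.
; The construction script registers the door mesh for highlighting and its shape for collision with the Interactable component.
; Completed interactions toggle between Open and Close, which set the open flag and target yaw.
; Tick continuously eases the door's relative yaw toward that target with FInterpTo.
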(event OnInteractionCompleted(Interactable)
  (params (FinishedInteractionType :type EInteractableType%20Enum :default "EIT_Hold") (FinishTime :type Float%20%28single-precision%29))
  (if (Variables|Default|GetIs%20Opened)
    (CallFunction|Close)
    (else
      (CallFunction|Open))))

(event EventTick
  (params (DeltaSeconds :type Float%20%28single-precision%29))
  (Transformation|SetRelativeRotation (Variables|Default|GetDoor) (Math|Rotator|MakeRotator 0.0 0.0 (Math|Interpolation|FInterpTo (.yaw (Variables|/Script/Engine.SceneComponent|GetRelativeRotation (Variables|Default|GetDoor))) (Variables|Default|GetTarget%20Yaw) DeltaSeconds 5.0)) false false))

(fn ConstructionScript
  (bind _interactable (Variables|Default|GetInteractable))
  (Class|ActorInteractableComponent|AddHighlightableMesh _interactable (Variables|Default|GetDoor))
  (Class|ActorInteractableComponent|AddCollisionShape _interactable (Variables|Default|GetDoor%20Shape)))

(fn Open
  (Variables|Default|SetIs%20Opened true)
  (Variables|Default|SetTarget%20Yaw 9e+01))

(fn Close
  (Variables|Default|SetIs%20Opened false)
  (Variables|Default|SetTarget%20Yaw 0.0))