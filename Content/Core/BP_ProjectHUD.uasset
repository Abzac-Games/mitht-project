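; BP_ProjectHUD is the project's HUD, managing the in-game widget and the result table shown when the game completes.
; On BeginPlay it shows the in-game widget in game-only input and pre-creates the result table.
; The game state's OnGameComplete event swaps to the table with UI input and a centered cursor.
; It also sets the displayed component name and provides formatted scenario name and elapsed-time text.
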(event Custom|On%20Game%20Complete
  (bind _result_table (Variables|Default|GetResult%20Table))
  (bind _playerowner (Variables|Default|GetPlayerOwner))
  (Widget|RemovefromParent (Variables|Default|GetIn%20Game))
  (UserInterface|Viewport|AddtoViewport _result_table 0)
  (Input|SetInputModeUIOnly _playerowner _result_table "DoNotLock")
  (Variables|/Script/Engine.PlayerController|SetbShowMouseCursor _playerowner true)
  (Utilities|CenterMouse))

(event EventBeginPlay
  (bind _playerowner (Variables|Default|GetPlayerOwner))
  (bind _playerowner_2 (Variables|Default|GetPlayerOwner))
  (EventDispatchers|AssignOnGameComplete (Variables|Default|GetGame%20State) (delegate Custom|On%20Game%20Complete))
  (Utilities|FlowControl|Sequence
    (:then_0
      (bind _returnvalue (UserInterface|CreateWidget "/Game/UI/In_Game/WBP_In_Game.WBP_In_Game_C" _playerowner))
      (bind _output_get (Variables|Default|SetIn%20Game _returnvalue))
      (UserInterface|Viewport|AddtoViewport _output_get 0)
      (Input|SetInputModeGameOnly _playerowner_2)
      (Variables|/Script/Engine.PlayerController|SetbShowMouseCursor _playerowner_2 false))
    (:then_1
      (bind _returnvalue_2 (UserInterface|CreateWidget "/Game/UI/In_Game/WBP_In_Game_Result_Table.WBP_In_Game_Result_Table_C" _playerowner))
      (Variables|Default|SetResult%20Table _returnvalue_2))))

(event EventSetComponentName
  (params (ComponentName :type Text%20%28by%20ref%29))
  (Variables|/Game/UI/In_Game/WBP_In_Game.WBP_In_Game_C|SetComponentName (Variables|Default|GetIn%20Game) ComponentName))

(event EventRemoveComponentName
  (Variables|/Game/UI/In_Game/WBP_In_Game.WBP_In_Game_C|SetComponentName (Variables|Default|GetIn%20Game) (Utilities|Text|MakeLiteralText "")))

(fn ConstructionScript
  (bind _asbp_gs_project (Utilities|Casting|CastToBP_GS_Project (Game|GetGameState)))
  (Variables|Default|SetGame%20State _asbp_gs_project))

(fn GetScenarioName
  (bind _game_state (Variables|Default|GetGame%20State))
  (bind _game_instance (Variables|/Game/Core/BP_GS_Project.BP_GS_Project_C|GetGame%20Instance _game_state))
  (bind _game_scenario (Variables|/Game/Core/BP_ProjectGameInstance.BP_ProjectGameInstance_C|GetGame%20Scenario _game_instance))
  (Utilities|IsValid _game_scenario
    (:Is%20Valid
      (return (Class|KismetTextLibrary|TexttoUpper (Utilities|Text|ToText(String) (Variables|/Game/Data/Initial/Blueprints/BP_Scenario.BP_Scenario_C|GetName _game_scenario)))))
    (:Is%20Not%20Valid
      (return (Class|KismetTextLibrary|TexttoUpper (Utilities|Text|MakeLiteralText "Название сценария"))))))

(fn GetGameSeconds
  (return (Utilities|Text|ToText(Integer) (Math|Integer|%(Integer) (Default|GetGameTime (Variables|Default|GetGame%20State)) (Variables|Default|GetSeconds%20in%20Minute)) false true 2 2)))

(fn GetGameMinutes
  (bind _seconds_in_minute (Variables|Default|GetSeconds%20in%20Minute))
  (return (Utilities|Text|ToText(Integer) (Math|Integer|%(Integer) (/ (Default|GetGameTime (Variables|Default|GetGame%20State)) _seconds_in_minute) _seconds_in_minute) false true 2 2)))

(fn GetGameHours
  (bind _seconds_in_minute (Variables|Default|GetSeconds%20In%20Minute))
  (return (Utilities|Text|ToText(Integer) (/ (Default|GetGameTime (Variables|Default|GetGame%20State)) (* _seconds_in_minute _seconds_in_minute)))))