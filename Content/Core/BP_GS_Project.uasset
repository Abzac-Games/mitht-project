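; Game state Blueprint that ends a timed scenario by pausing the game and firing OnGameComplete.
; Construction caches the project game instance, and Tick polls CheckTime while a GameScenario is valid, completing only once through a DoOnce.
; CheckTime's graph compares the scenario's non-zero TimeToComplete with truncated server world time, but that expression appears unconnected.
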(event EventTick
  (params (DeltaSeconds :type Float%20%28single-precision%29))
  (Utilities|IsValid (Variables|/Game/Core/BP_ProjectGameInstance.BP_ProjectGameInstance_C|GetGame%20Scenario (Variables|Default|GetGame%20Instance))
    (:Is%20Valid
      (if (Utilities|CheckTime)
        (Utilities|FlowControl|DoOnce false
          (:Completed
            (Game|SetGamePaused true)
            (Default|CallOnGameComplete self)))))))

(fn ConstructionScript
  (bind _asbp_project_game_instance (Utilities|Casting|CastToBP_ProjectGameInstance (Game|GetGameInstance)))
  (Variables|Default|SetGame%20Instance _asbp_project_game_instance))

(fn GetGameTime
  (return (Math|Float|Truncate (GameState|GetServerWorldTimeSeconds))))