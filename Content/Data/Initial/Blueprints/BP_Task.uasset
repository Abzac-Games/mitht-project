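; BP_Task is a data Blueprint that represents a task with an ID, a name and a collection of steps.
; Accessor functions read the ID, read and write the name, and return, add to, remove from or clear the steps.
; The ID has a getter but no setter here, and the file contains no execution logic for the steps.
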(fn GetID
  (return (Variables|Default|GetID)))

(fn GetSteps
  (return (Variables|Default|GetSteps)))

(fn AddStep
  (params (Step :type BP%20Step%20Soft%20Object%20Reference%20%28by%20ref%29))
  (Utilities|Array|Add (Variables|Default|GetSteps) Step))

(fn DeleteStep
  (params (Step :type BP%20Step%20Soft%20Object%20Reference%20%28by%20ref%29))
  (Utilities|Array|RemoveItem (Variables|Default|GetSteps) Step))

(fn ClearSteps
  (Utilities|Array|Clear (Variables|Default|GetSteps)))

(fn GetName
  (return (Variables|Default|GetName)))

(fn SetName
  (params (Name :type String))
  (Variables|Default|SetName Name))