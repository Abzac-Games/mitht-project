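; BP_Scenario is a data Blueprint that describes one scenario: its ID, name, main goal, description, equipment, time to complete and list of tasks.
; Boolean options record what can be seen or highlighted, such as tasks, steps, result deviation, element names and current-step elements.
; Plain getters and setters expose the fields, with add, delete and clear functions for tasks and a read-only accessor for the ID.
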(fn GetID
  (return (Variables|Default|GetID)))

(fn GetTasks
  (return (Variables|Default|GetTasks)))

(fn AddTask
  (params (Task :type BP%20Task%20Soft%20Object%20Reference%20%28by%20ref%29))
  (Utilities|Array|Add (Variables|Default|GetTasks) Task))

(fn DeleteTask
  (params (Task :type BP%20Task%20Soft%20Object%20Reference%20%28by%20ref%29))
  (Utilities|Array|RemoveItem (Variables|Default|GetTasks) Task))

(fn ClearTasks
  (Utilities|Array|Clear (Variables|Default|GetTasks)))

(fn GetEquipment
  (return (Variables|Default|GetEquipment)))

(fn SetEquipment
  (params (Equipment :type Actor%20Soft%20Object%20Reference))
  (Variables|Default|SetEquipment Equipment))

(fn GetName
  (return (Variables|Default|GetName)))

(fn SetName
  (params (Name :type String))
  (Variables|Default|SetName Name))

(fn GetMainGoal
  (return (Variables|Default|GetMain%20Goal)))

(fn SetMainGoal
  (params (Main%20Goal :type String))
  (Variables|Default|SetMain%20Goal Main%20Goal))

(fn GetDescription
  (return (Variables|Default|GetDescription)))

(fn SetDescription
  (params (Description :type String))
  (Variables|Default|SetDescription Description))

(fn GetTimetoComplete
  (return (Variables|Default|GetTime%20to%20complete)))

(fn SetTimetoComplete
  (params (Time%20to%20complete :type Int%2032%20Range%20Structure))
  (Variables|Default|SetTime%20to%20complete Time%20to%20complete))

(fn IfCanSeeDeviationfromResult
  (return (Variables|Default|GetCan%20see%20Deviation%20from%20Result)))

(fn SetCanSeeDeviationfromResult
  (params (Can%20see%20Deviation%20from%20Result :type Boolean))
  (Variables|Default|SetCan%20see%20Deviation%20from%20Result Can%20see%20Deviation%20from%20Result))

(fn IfCanSeeTasks
  (return (Variables|Default|GetCan%20see%20Tasks)))

(fn SetCanSeeTasks
  (params (Can%20see%20Tasks :type Boolean))
  (Variables|Default|SetCan%20see%20Tasks Can%20see%20Tasks))

(fn IfCanSeeSteps
  (return (Variables|Default|GetCan%20see%20Steps)))

(fn SetCanSeeSteps
  (params (Can%20see%20Steps :type Boolean))
  (Variables|Default|SetCan%20see%20Steps Can%20see%20Steps))

(fn IfHighlightElementsName
  (return (Variables|Default|GetHighlight%20Elements%20Name)))

(fn SetHighlightElementsName
  (params (Highlight%20Elements%20Name :type Boolean))
  (Variables|Default|SetHighlight%20Elements%20Name Highlight%20Elements%20Name))

(fn IfHighlightCurrentStepElements
  (return (Variables|Default|GetHighlight%20current%20Step%20Elements)))

(fn SetHighlightCurrentStepElements
  (params (Highlight%20current%20Step%20Elements :type Boolean))
  (Variables|Default|SetHighlight%20current%20Step%20Elements Highlight%20current%20Step%20Elements))