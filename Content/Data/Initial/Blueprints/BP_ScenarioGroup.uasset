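; BP_ScenarioGroup is a data container that represents a named group of scenarios with an ID.
; It holds a Scenarios collection, with functions to add, delete, clear and return its entries.
; Accessor functions expose the ID and Name, and only the Name has a setter.
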(fn GetID
  (return (Variables|Default|GetID)))

(fn GetScenarios
  (return (Variables|Default|GetScenarios)))

(fn AddScenario
  (params (Scenario :type BP%20Scenario%20Soft%20Object%20Reference%20%28by%20ref%29))
  (Utilities|Array|Add (Variables|Default|GetScenarios) Scenario))

(fn DeleteScenario
  (params (Scenario :type BP%20Scenario%20Soft%20Object%20Reference%20%28by%20ref%29))
  (Utilities|Array|RemoveItem (Variables|Default|GetScenarios) Scenario))

(fn ClearScenarios
  (Utilities|Array|Clear (Variables|Default|GetScenarios)))

(fn GetName
  (return (Variables|Default|GetName)))

(fn SetName
  (params (Name :type String))
  (Variables|Default|SetName Name))