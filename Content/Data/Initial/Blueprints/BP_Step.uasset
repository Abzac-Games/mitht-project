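; BP_Step is a data holder for one step, with an ID, a name, a link to a previous step and a collection of component states.
; Accessor functions expose these fields, with the ID having only a getter.
; Component states can be added, removed or cleared, and the previous-step reference allows steps to be chained backwards.
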(fn GetID
  (return (Variables|Default|GetID)))

(fn GetPreviousStep
  (return (Variables|Default|GetPreious%20Step)))

(fn SetPreviousStep
  (params (Preious%20Step :type BP%20Step%20Soft%20Object%20Reference))
  (Variables|Default|SetPreious%20Step Preious%20Step))

(fn GetComponentSteps
  (return (Variables|Default|GetComponent%20States)))

(fn AddComponentState
  (params (Component%20State :type BP%20Component%20State%20Soft%20Object%20Reference%20%28by%20ref%29))
  (Utilities|Array|Add (Variables|Default|GetComponent%20States) Component%20State))

(fn DeleteComponentState
  (params (Component%20State :type BP%20Component%20State%20Soft%20Object%20Reference%20%28by%20ref%29))
  (Utilities|Array|RemoveItem (Variables|Default|GetComponent%20States) Component%20State))

(fn ClearComponentSteps
  (Utilities|Array|Clear (Variables|Default|GetComponent%20States)))

(fn GetName
  (return (Variables|Default|GetName)))

(fn SetName
  (params (Name :type String))
  (Variables|Default|SetName Name))